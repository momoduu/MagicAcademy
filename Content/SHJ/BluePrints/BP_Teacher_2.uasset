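; BP_Teacher_2 is a teacher Blueprint that reveals the player's timer bar when its state machine enters Study.
; BeginPlay caches the player's BP_ThirdPersonCharacter.
; Tick polls the Fsm state and, while in Study with the TimerWidget hidden, waits three seconds before making it visible.
; The visibility check stands in for a run-once guard, and nothing here hides the timer again.
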(event EventBeginPlay
  ;[1 1 1] Player 담아 놓기
  (bind _asbp_third_person_character (Utilities|Casting|CastToBP_ThirdPersonCharacter (Game|GetPlayerCharacter 0)))
  (Variables|Default|SetAs%20BP%20Third%20Person%20Character _asbp_third_person_character))

(event Collision|EventActorBeginOverlap
  (params (OtherActor :type Actor%20Object%20Reference)))

(event EventTick
  (params (DeltaSeconds :type Float%20%28single-precision%29))
  (bind _as_bp_third_person_character (Variables|Default|GetAs%20BP%20Third%20Person%20Character))
  (bind _timerwidget (Variables|/Game/ThirdPerson/Blueprints/BP_ThirdPersonCharacter.BP_ThirdPersonCharacter_C|GetTimerWidget _as_bp_third_person_character))
  ;[1 1 1] 만약 Study 상태가 되었다면..
  (if (Utilities|Enum|Equal(Enum) (Variables|/Script/FinalProject.TeacherFSM|GetmState (Variables|Default|Getfsm)) "Study")
    ;[1 1 1] Timer Bar 한번만 실행
    (if (not (Rendering|IsVisible _timerwidget))
      (Utilities|FlowControl|Delay 3.0)
      (Rendering|SetVisibility _timerwidget true false))))

(fn ConstructionScript)