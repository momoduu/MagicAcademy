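; Flower herb pickup that the player can click to inspect or interact with to collect.
; Cursor hover drives a "Select" material highlight; clicking opens a herb widget and, behind a DoOnce, moves the flower onto the player camera for axis-driven rotation.
; Detach returns it to its saved transform and resets the gate.
; Box overlap handles interactable registration, and StartInteractive adds it to inventory, hiding the mesh and disabling collision on success.
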(event OnBeginCursorOver(Flower)
  (params (TouchedComponent :type Primitive%20Component%20Object%20Reference))
  ;[1 1 1] mouse cursor actor  선택되는 머티리얼
  (if (not (Variables|Default|Getinspecting))
    (Rendering|Material|SetScalarParameterValueonMaterials (Variables|Default|GetFlower) "Select" 1.0)))

(event OnEndCursorOver(Flower)
  (params (TouchedComponent :type Primitive%20Component%20Object%20Reference))
  ;[1 1 1] mouse cursor actor  선택되는 머티리얼
  (Rendering|Material|SetScalarParameterValueonMaterials (Variables|Default|GetFlower) "Select" 0.0))

(event OnComponentBeginOverlap(flowerBox)
  (params (OverlappedComponent :type Primitive%20Component%20Object%20Reference) (OtherActor :type Actor%20Object%20Reference) (OtherComp :type Primitive%20Component%20Object%20Reference) (OtherBodyIndex :type Integer) (bFromSweep :type Boolean) (SweepResult :type Hit%20Result%20Structure%20%28by%20ref%29))
  (Class|BPICharacter|SetInteractableObject(Message) OtherActor self))

(event OnComponentEndOverlap(flowerBox)
  (params (OverlappedComponent :type Primitive%20Component%20Object%20Reference) (OtherActor :type Actor%20Object%20Reference) (OtherComp :type Primitive%20Component%20Object%20Reference) (OtherBodyIndex :type Integer))
  (Class|BPICharacter|SetInteractableObject(Message) (Variables|Default|GetflowerBox) self))

(event Custom|Detach
  (bind _returnvalue (Transformation|GetActorTransform))
  ;[1 1 1] Cancel Clicked
  (Variables|Default|Setinspecting false)
  ;[1 1 1] 기존 위치, 회전 상태로 되돌리기
  (Transformation|DetachFromActor self "KeepWorld" "KeepWorld" "KeepWorld")
  (Input|DisableInput (Game|GetPlayerController 0))
  (Components|MoveComponentTo (Variables|Default|GetDefaultSceneRoot) (Variables|Default|GetOri%20Loc) (Variables|Default|GetOri%20Rot) false false 0.3 false)
  (Utilities|FlowControl|DoOnce false) ; enters at Reset
)

(event Collision|EventActorBeginOverlap
  (params (OtherActor :type Actor%20Object%20Reference))
  (|CallParentFunction OtherActor) ; This node is disabled and will not be called.\nDrag off pins to build functionality.
)

(event EventTick
  (params (DeltaSeconds :type Float%20%28single-precision%29))
  (|CallParentFunction DeltaSeconds) ; This node is disabled and will not be called.\nDrag off pins to build functionality.
)

(event EventStartInteractive
  (params (Interacting%20Character :type Character%20Object%20Reference))
  ;[1 1 1] Aloe를 Inventory에 추가하기
  (if (Variables|Default|GetHas%20Herbs)
    (|CallParentFunction Interacting%20Character)
    (bind _output_get (Variables|Default|SetInteracting%20Character Interacting%20Character))
    (bind _collected (Class|BPICharacter|AddtoInventory(Message) _output_get (Utilities|Struct|MakeResourceData "Flower" "/Game/SHJ/Image/img_Flower.img_Flower" "Herbs : Flower " 0 0 0)))
    (if _collected
      (Development|SetHiddeninGame (Variables|Default|GetFlower) true false)
      (Variables|Default|SetHas%20Herbs false)
      (Collision|SetCollisionEnabled (Variables|Default|GetflowerBox) "NoCollision"))))

(event EventBeginPlay
  (|CallParentFunction)
  (bind _asbp_third_person_character (Utilities|Casting|CastToBP_ThirdPersonCharacter (Game|GetPlayerCharacter 0)))
  (Variables|Default|SetAs%20BP%20Third%20Person%20Character _asbp_third_person_character))

(event MouseInput|EventActorOnClicked
  (params (ButtonPressed :type Key%20Structure :default "None"))
  (bind _returnvalue (Transformation|GetActorTransform))
  ;[1 1 1] Actor Clicked
  (Variables|/Game/ThirdPerson/Blueprints/BP_ThirdPersonCharacter.BP_ThirdPersonCharacter_C|SetbTimeLine (Variables|Default|GetAs%20BP%20Third%20Person%20Character) true)
  (bind _returnvalue_2 (UserInterface|CreateWidget "/Game/SHJ/UI/Exam2_UI/BP_Herbs_Flower.BP_Herbs_Flower_C"))
  (UserInterface|Viewport|AddtoViewport _returnvalue_2 0)
  (Utilities|FlowControl|DoOnce false
    (:Completed
      ;[1 1 1] 기존 Actor의 위치, 회전 값 저장
      (Variables|Default|SetOri%20Loc (.location _returnvalue))
      (Variables|Default|SetOri%20Rot (.rotation _returnvalue))
      ;[1 1 1] Player Cam에 선택된 Actor 붙이기
      (Variables|Default|Setinspecting true)
      (Transformation|AttachComponentToComponent self (Variables|/Script/Engine.PlayerCameraManager|GetTransformComponent (Game|GetPlayerCameraManager 0)) "None" "KeepWorld" "KeepWorld" "KeepWorld" true)
      ;[1 1 1] 설정한 위치로 세팅
      (Components|MoveComponentTo (Variables|Default|GetDefaultSceneRoot) "417.000000,209.000000,-119.000000" "0,90.000000, 0" false false 0.3 false)
      (Input|EnableInput (Game|GetPlayerController 0)))))

(event Input|AxisEvents|InputAxisActorTurn
  (params (AxisValue :type Float%20%28single-precision%29))
  ;[1 1 1] 선택된 actor 마우스로 검사하기
  (Transformation|AddLocalRotation (Variables|Default|GetDefaultSceneRoot) (Math|Rotator|MakeRotator 0.0 0.0 AxisValue) false false))

(event Input|AxisEvents|InputAxisActorLookUP
  (params (AxisValue :type Float%20%28single-precision%29))
  ;[1 1 1] 선택된 actor 마우스로 검사하기
  (Transformation|AddLocalRotation (Variables|Default|GetDefaultSceneRoot) (Math|Rotator|MakeRotator AxisValue 0.0 0.0) false false))

(fn ConstructionScript
  (|CallParentFunction))