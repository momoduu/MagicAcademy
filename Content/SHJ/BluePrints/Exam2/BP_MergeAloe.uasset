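; BP_MergeAloe is an actor that reveals a hidden aloe merge component and drops it a short distance.
; BeginPlay hides the MergeAloe component and stores the actor's starting location.
; The Falling event waits briefly, shows MergeAloe, makes an attach call, then uses MoveComponentTo to quickly move the root to a point below the saved location.
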(event Custom|Falling
  ;[1 1 1] 원하는 위치로 이동
  (Utilities|FlowControl|Delay 2.0)
  (Development|SetHiddeninGame (Variables|Default|GetmergeAloe) false false)
  (Transformation|AttachComponentToComponent self 0 "None" "KeepRelative" "KeepRelative" "KeepRelative" true)
  (Components|MoveComponentTo (Variables|Default|GetDefaultSceneRoot) (Math|Vector|MakeVector (Variables|Default|GetReturn%20Value%20X) (Variables|Default|GetReturn%20Value%20Y) (- (Variables|Default|GetReturn%20Value%20Z) 9e+01)) "0, 0, 0" false false 0.3 false))

(event EventBeginPlay
  (bind _returnvalue (Transformation|GetActorLocation))
  ;[1 1 1] 현재 위치 저장
  (Development|SetHiddeninGame (Variables|Default|GetmergeAloe) true false)
  (Variables|Default|SetReturn%20Value%20X (.x _returnvalue))
  (Variables|Default|SetReturn%20Value%20Y (.y _returnvalue))
  (Variables|Default|SetReturn%20Value%20Z (.z _returnvalue)))

(event Collision|EventActorBeginOverlap
  (params (OtherActor :type Actor%20Object%20Reference)))

(event EventTick
  (params (DeltaSeconds :type Float%20%28single-precision%29)))

(fn ConstructionScript)