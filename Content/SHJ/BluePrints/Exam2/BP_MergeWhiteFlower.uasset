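; BP_MergeWhiteFlower is a white flower actor that stays hidden until it is triggered to appear and drop.
; BeginPlay hides the MergeFlower component and stores the actor's starting location and rotation.
; The Falling custom event waits briefly, reveals the flower, makes an attach call, then uses MoveComponentTo to lower the root quickly to a point below the saved location.
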(event Custom|Falling
  (Utilities|FlowControl|Delay 2.0)
  (Development|SetHiddeninGame (Variables|Default|GetmergeFlower) false false)
  ;[1 1 1] 원하는 위치로 이동
  (Transformation|AttachComponentToComponent self 0 "None" "KeepRelative" "KeepRelative" "KeepRelative" true)
  (Components|MoveComponentTo (Variables|Default|GetDefaultSceneRoot) (- (Variables|Default|GetReturn%20Value%20Location) "0,0,80.000000") "0, 0, 0" false false 0.3 false))

(event EventBeginPlay
  (bind _returnvalue (Transformation|GetActorTransform))
  ;[1 1 1] 현재 위치 저장
  (Development|SetHiddeninGame (Variables|Default|GetmergeFlower) true false)
  (Variables|Default|SetReturn%20Value%20Location (.location _returnvalue))
  (Variables|Default|SetReturn%20Value%20Rotation (.rotation _returnvalue)))

(event Collision|EventActorBeginOverlap
  (params (OtherActor :type Actor%20Object%20Reference)))

(event EventTick
  (params (DeltaSeconds :type Float%20%28single-precision%29)))

(fn ConstructionScript)