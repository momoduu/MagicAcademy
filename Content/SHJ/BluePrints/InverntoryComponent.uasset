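; Inventory component that holds a list of herb items and mirrors it in GameInstance_HJ.
; On BeginPlay it rebuilds its list from the game instance's saved InventoryItems through AddItemInit, which only appends locally.
; AddItem appends through the same function, then copies the whole list back to the game instance, so items can outlast the component.
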(event EventBeginPlay
  (bind _asgame_instance_hj (Utilities|Casting|CastToGameInstance_HJ (Game|GetGameInstance)))
  (if (> (Utilities|Array|Length (Variables|/Game/SHJ/UI/Struct/GameInstance_HJ.GameInstance_HJ_C|GetinventoryItems _asgame_instance_hj)) 0)
    (bind _result (Math|Integer|DecrementInt (Utilities|Array|Length (Variables|/Game/SHJ/UI/Struct/GameInstance_HJ.GameInstance_HJ_C|GetinventoryItems _asgame_instance_hj)))
      (:%20%20
        (for _index (range 0 _result)
          (CallFunction|AddItemInit (Utilities|Array|Get(acopy) (Variables|/Game/SHJ/UI/Struct/GameInstance_HJ.GameInstance_HJ_C|GetinventoryItems _asgame_instance_hj) _index)))))))

(event EventTick
  (params (DeltaSeconds :type Float%20%28single-precision%29)))

(fn AddItem
  (params (herbItem :type Resource%20Data%20Structure))
  ;[1 1 1] Add Item
  (CallFunction|AddItemInit herbItem)
  (bind _asgame_instance_hj (Utilities|Casting|CastToGameInstance_HJ (Game|GetGameInstance)))
  (Variables|/Game/SHJ/UI/Struct/GameInstance_HJ.GameInstance_HJ_C|SetinventoryItems _asgame_instance_hj (Variables|Default|Getitem)))

(fn AddItemInit
  (params (herbItem :type Resource%20Data%20Structure))
  (Utilities|Array|Add (Variables|Default|Getitem) herbItem))